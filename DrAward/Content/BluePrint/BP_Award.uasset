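; BP_Award is the player character, handling its lights, audio listener and death.
; On BeginPlay it moves the controller's audio listener to the HeadLight and turns both lights red in the "End" level if AwardGameInstance is not cleared.
; The first damage taken plays a death voice and ragdolls the mesh, then either spends a GameInstance Life and expires shortly after, or opens "End" when none remain.
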(event `self.ReceiveBeginPlay`
  (bind _asbp_award_controller (cast `/Game/BluePrint/BP_AwardController` (`self.GetController`))
    (:`then`
      (`PlayerController.SetAudioListenerOverride` :`self` _asbp_award_controller :`AttachToComponent` (`self.HeadLight`)))
    (:`CastFailed`
      _))
  (bind _returnvalue (`GameplayStatics.GetCurrentLevelName` true))
  (if (and (`KismetStringLibrary.EqualEqual_StrStr` _returnvalue "End") (not (`/Game/BluePrint/AwardGameInstance.IsClear` (cast `/Game/BluePrint/AwardGameInstance` (`GameplayStatics.GetGameInstance`) :!pure true))))
    (`LightComponent.SetLightColor` (`self.HeadLight`) (struct :`R` 1.0 :`A` 1.0) true)
    (`LightComponent.SetLightColor` (`self.PointLight`) (struct :`R` 1.0 :`A` 1.0) true)))

(event `self.ReceiveAnyDamage`
  (params (Damage :type "Float (single-precision)") (DamageType :type "DamageType Object Reference") (InstigatedBy :type "Controller Object Reference") (DamageCauser :type "Actor Object Reference"))
  (bind _mesh (`self.Mesh`))
  (bind _asaward_game_instance (cast `/Game/BluePrint/AwardGameInstance` (`GameplayStatics.GetGameInstance`) :!pure true))
  (bind _life (`/Game/BluePrint/AwardGameInstance.Life` _asaward_game_instance))
  (`/Engine/EditorBlueprintResources/StandardMacros.DoOnce` false
    (:`Completed`
      (`GameplayStatics.SpawnSound2D` "/Game/Audio/death_voice.death_voice" 1.0 1.0 0.0 null)
      (`|ExecutionSequence`
        (:`then_0`
          ;[1 1 1] Ragdoll処理
          (`CharacterMovementComponent.DisableMovement` (`self.CharacterMovement`))
          (`PrimitiveComponent.SetCollisionProfileName` _mesh "Ragdoll" true)
          (`PrimitiveComponent.SetSimulatePhysics` _mesh true))
        (:`then_1`
          ;[1 1 1] Life処理
          (if (> _life 0)
            (set `/Game/BluePrint/AwardGameInstance.Life` (- _life 1) _asaward_game_instance)
            (`self.SetLifeSpan` 3.0)
            (else
              (`KismetSystemLibrary.Delay` 3.0)
              (`GameplayStatics.OpenLevel` "End"))))))))

(fn `UserConstructionScript`)