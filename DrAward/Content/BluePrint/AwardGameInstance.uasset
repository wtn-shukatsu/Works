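; AwardGameInstance is a Game Instance that holds the game's save data and provides a shared loading screen.
; On Init it loads a BP_AwardSaveGame from the award slot and flags that data exists, or creates a fresh save object without writing it to disk.
; Loading adds a W_Loading widget to the viewport and returns it with the loading duration, leaving its removal to the caller.
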(event `self.ReceiveInit`
  (bind _returnvalue (`GameplayStatics.LoadGameFromSlot` (`self.AwardSlotName`)))
  (bind _asbp_award_save_game (cast `/Game/BluePrint/BP_AwardSaveGame` _returnvalue)
    (:`then`
      (set `self.GameData` _asbp_award_save_game)
      (set `self.IsGameData` true))
    (:`CastFailed`
      (bind _returnvalue_2 (`GameplayStatics.CreateSaveGameObject` "/Game/BluePrint/BP_AwardSaveGame.BP_AwardSaveGame_C"))
      (set `self.GameData` _returnvalue_2))))

(fn `Loading`
  (returns (Dulation :type "Float (double-precision)") (ReturnValue :type "/Game/UI/W_Loading Object Reference"))
  (bind _returnvalue (`|CreateWidget` "/Game/UI/W_Loading.W_Loading_C"))
  (`UserWidget.AddToViewport` _returnvalue 0)
  (return (`self.LoadingTime`) _returnvalue))