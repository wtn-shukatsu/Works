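; Blueprint function library with small helpers for award damage and number display text.
; DamageAward casts the given object to BP_Award and applies fixed damage to it.
; AppendZero turns an integer into text, prefixing a zero when it is 9 or below.
; StageNumToText strips a five-character prefix from the game instance's Stage string, showing that number if IsClear is set and one less otherwise.
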(fn `AppendZero`
  (params (InInt :type Integer))
  (returns (ReturnValue :type Text))
  (return (select `bool` (> InInt 9) :`false` (`KismetTextLibrary.Conv_StringToText` (`KismetStringLibrary.Concat_StrStr` "0" (`KismetStringLibrary.Conv_IntToString` InInt))) :`true` (`KismetTextLibrary.Conv_IntToText` InInt))))

(fn `DamageAward`
  (params (Object :type "Object Object Reference"))
  (bind _asbp_award (cast `/Game/BluePrint/BP_Award` Object))
  (`GameplayStatics.ApplyDamage` _asbp_award 100.0))

(fn `StageNumToText`
  (params (AwardGameInstance :type "/Game/BluePrint/AwardGameInstance Object Reference"))
  (returns (StageNum :type Text))
  (bind _returnvalue (`KismetStringLibrary.RightChop` (`KismetStringLibrary.Conv_NameToString` (`/Game/BluePrint/AwardGameInstance.Stage` AwardGameInstance)) 5))
  (return (select `bool` (`/Game/BluePrint/AwardGameInstance.IsClear` AwardGameInstance) :`false` (`KismetTextLibrary.Conv_IntToText` (- (`KismetStringLibrary.Conv_StringToInt` _returnvalue) 1)) :`true` (`KismetTextLibrary.Conv_StringToText` _returnvalue))))